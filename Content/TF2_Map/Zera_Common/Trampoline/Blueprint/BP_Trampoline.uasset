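; BP_Trampoline is a trampoline actor that launches the player character straight up.
; When a BP_CPS1999_Playable overlaps its Box, LaunchCharacter replaces the character's velocity with a vertical one equal to JumpHeight, cancelling horizontal motion.
; The construction script offsets an Arrow component upward by the same JumpHeight value, which is a launch speed rather than the actual apex height.
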(event OnComponentBeginOverlap(Box)
  (params (OverlappedComponent :type Primitive%20Component%20Object%20Reference) (OtherActor :type Actor%20Object%20Reference) (OtherComp :type Primitive%20Component%20Object%20Reference) (OtherBodyIndex :type Integer) (bFromSweep :type Boolean) (SweepResult :type Hit%20Result%20Structure%20%28by%20ref%29))
  (bind _asbp_cps1999_playable (Utilities|Casting|CastToBP_CPS1999_Playable OtherActor))
  (Character|LaunchCharacter _asbp_cps1999_playable (Math|Vector|MakeVector 0.0 0.0 (Variables|Default|GetJumpHeight)) true true))

(fn ConstructionScript
  (Transformation|SetRelativeLocation (Variables|Default|GetArrow) (Math|Vector|MakeVector 0.0 0.0 (Variables|Default|GetJumpHeight)) false false))