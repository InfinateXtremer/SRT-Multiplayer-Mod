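; Flag pickup for the KOTF mode: players take or steal it by overlap, and its holder scores over time.
; The server handles pickups with a short cooldown, then multicasts attachment to the pelvis socket and optional custom-depth outline, tinted by session color via post-process.
; A looping server timer adds points to the holder's PlayerState and reloads the level via servertravel at WinCount.
; RespawnFlag restores the transform saved in the construction script.
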(event OnComponentBeginOverlap(Sphere)
  (params (OverlappedComponent :type Primitive%20Component%20Object%20Reference) (OtherActor :type Actor%20Object%20Reference) (OtherComp :type Primitive%20Component%20Object%20Reference) (OtherBodyIndex :type Integer) (bFromSweep :type Boolean) (SweepResult :type Hit%20Result%20Structure%20%28by%20ref%29))
  (Networking|SwitchHasAuthority
    (:Authority
      (bind _asbp_cps1999_playable (Utilities|Casting|CastToBP_CPS1999_Playable OtherActor))
      (CallFunction|PickupServer _asbp_cps1999_playable (Pawn|GetController _asbp_cps1999_playable)))))

(event Custom|PickupServer
  (params (Player :type BP%20CPS1999%20Playable%20Object%20Reference) (PlayerController :type Controller%20Object%20Reference))
  (if (not (Variables|Default|GetInCooldown))
    (Variables|Default|SetInCooldown true)
    (CallFunction|PickupMulticast Player (Variables|Default|GetCurrent%20Flag%20Holder) PlayerController) ; Tell everyone else someone has picked me up!
    (bind _output_get (Variables|Default|SetCurrent%20Flag%20Holder Player))
    (bind _askotf_player_state (Utilities|Casting|CastToKOTF_PlayerState (Variables|/Script/Engine.Pawn|GetPlayerState _output_get)))
    (Variables|Default|SetFlag%20Holder's%20State _askotf_player_state)
    (CallFunction|PointCount PlayerController)
    (Utilities|FlowControl|Delay 2.0)
    (Variables|Default|SetInCooldown false)
    (Default|CallNotifyPickedUp)))

(event Custom|PointCount
  (params (Player%20Controller :type Controller%20Object%20Reference))
  (Variables|Default|SetFlagHolder_PlayerController Player%20Controller)
  (Networking|SwitchHasAuthority
    (:Authority
      (bind _returnvalue (Utilities|Time|SetTimerbyEvent (delegate Custom|PointCounter) 1.0 true)))))

(event Custom|EndRoundServer
  (bind _returnvalue (Game|GetCurrentLevelName true))
  (Development|ExecuteConsoleCommand (Utilities|String|Append "servertravel " _returnvalue)))

(event Custom|PickupMulticast
  (params (Player :type BP%20CPS1999%20Playable%20Object%20Reference) (PreviousPlayer :type BP%20CPS1999%20Playable%20Object%20Reference) (PlayerController :type Controller%20Object%20Reference))
  (bind _mesh (Variables|/Script/Engine.Character|GetMesh Player))
  (Utilities|IsValid PreviousPlayer
    (:Is%20Valid
      (Rendering|SetRenderCustomDepth (Variables|/Script/Engine.Character|GetMesh PreviousPlayer) false) ; This disables outline for player who just lost the flag
    )
    (:Is%20Not%20Valid
      _))
  (Utilities|FlowControl|Sequence
    (:then_0
      (if (Variables|Modularity|GetCharacterOutline?)
        (Rendering|SetRenderCustomDepth _mesh true))
      (Transformation|AttachComponentToComponent (Variables|Default|GetDefaultSceneRoot) _mesh "None" "SnapToTarget" "KeepRelative" "KeepRelative" true)
      (Transformation|AttachComponentToComponent (Variables|Default|GetPickup) _mesh "socket_pelvis" "SnapToTarget" "KeepRelative" "KeepRelative" true)
      (bind _output_get (Variables|Default|SetFlagHolderMesh (Variables|/Script/Engine.Character|GetMesh Player)))
      (Audio|SpawnSoundAttached "/Game/GameModes/KOTF/Blueprints/Flag/Sound/PickedUp.PickedUp" _output_get "None" "0, 0, 0" "0, 0, 0" "SnapToTarget" false 1.0 1.0 0.0 "/Game/GameModes/KOTF/Blueprints/Flag/Sound/GeneralSpeech.GeneralSpeech"))
    (:then_1
      (Variables|/Script/Engine.RotatingMovementComponent|SetRotationRate (Variables|Default|GetRotatingMovement) "0, 0, 0") ; Stop rotation after picking up
      (Transformation|SetRelativeRotation (Variables|Default|GetDefaultSceneRoot) "0, 0, 0" false false)
      (Transformation|SetRelativeRotation (Variables|Default|GetPickup) "90.000000,90.000000,90.000000" false false))
    (:then_2
      (if (Variables|Default|GetPlayerColorSpecificOutline?)
        (CallFunction|SetPostProcess Player)))))

(event Custom|PointCounter
  (bind _flag_holder_s_state (Variables|Default|GetFlag%20Holder's%20State))
  (Utilities|IsValid _flag_holder_s_state ; If doesn't exist, we can respawn flag
    (:Is%20Valid
      (if (not (Variables|Default|GetRoundFinished?)) ; Finish counting after round ends
        (if (== (Variables|/Game/GameModes/KOTF/MultiplayerMode/KOTF_PlayerState.KOTF_PlayerState_C|GetPoints _flag_holder_s_state) (Variables|Modularity|GetWin%20Count))
          (Utilities|Time|ClearandInvalidateTimerbyHandle (stale Custom|PointCount _returnvalue))
          (Variables|Default|SetRoundFinished? true)
          (CallFunction|EndRoundServer)
          (else
            (bind _output_get (Variables|/Game/GameModes/KOTF/MultiplayerMode/KOTF_PlayerState.KOTF_PlayerState_C|SetPoints _flag_holder_s_state (+ 1 (Variables|/Game/GameModes/KOTF/MultiplayerMode/KOTF_PlayerState.KOTF_PlayerState_C|GetPoints _flag_holder_s_state))))
            (if (== _output_get (Math|Float|Truncate (/ (Math|Conversions|ToFloat(Integer) (Variables|Modularity|GetWin%20Count)) 1.2)))
              (Audio|SpawnSoundAttached "/Game/GameModes/KOTF/Blueprints/Flag/Sound/PickedUp.PickedUp" (Variables|Default|GetFlagHolderMesh) "None" "0, 0, 0" "0, 0, 0" "SnapToTarget" false 1.0 1.0 0.0 "/Game/GameModes/KOTF/Blueprints/Flag/Sound/GeneralSpeech.GeneralSpeech"))))))))

(event Custom|RespawnFlag
  (bind _sphere (Variables|Default|GetSphere))
  (bind _pickup (Variables|Default|GetPickup))
  (bind _defaultsceneroot (Variables|Default|GetDefaultSceneRoot))
  (Utilities|Time|ClearandInvalidateTimerbyHandle (stale Custom|PointCount _returnvalue))
  (Transformation|DetachFromActor "KeepRelative" "KeepRelative" "KeepRelative")
  (Utilities|FlowControl|Sequence
    (:then_0
      (Transformation|AttachComponentToComponent _pickup _defaultsceneroot "None" "SnapToTarget" "SnapToTarget" "SnapToTarget" true)
      (Transformation|SetRelativeLocationAndRotation _pickup (Variables|Modularity|GetPick-Up%20Location) (Variables|Modularity|GetPick-Up%20Rotation) false false)
      (Transformation|SetRelativeScale3D _pickup (Variables|Modularity|GetPick-Up%20Scale))
      (Transformation|SetActorTransform (Variables|Default|GetRespawnLocation))
      (Variables|/Script/Engine.RotatingMovementComponent|SetRotationRate (Variables|Default|GetRotatingMovement) (Variables|Modularity|GetRotation%20Rate))
      (Default|CallNotifyRespawned))
    (:then_1
      (Transformation|AttachComponentToComponent _sphere _defaultsceneroot "None" "SnapToTarget" "SnapToTarget" "SnapToTarget" true)
      (Transformation|SetRelativeLocationAndRotation _sphere (Variables|Modularity|GetPick-Up%20Collision%20Location) (Variables|Modularity|GetPick-Up%20Collision%20Rotation) false false))))

(event Custom|SetPostProcess
  (params (Player :type BP%20CPS1999%20Playable%20Object%20Reference))
  (bind _askotf_player_state (Utilities|Casting|CastToKOTF_PlayerState (Variables|/Script/Engine.Pawn|GetPlayerState Player)))
  (Utilities|IsValid (Variables|Default|GetPP_Material)
    (:Is%20Valid
      (Rendering|Material|SetVectorParameterValue (stale _returnvalue) "OutlineColor" (Variables|/Game/Multiplayer/Blueprints/Overrides/Multiplayer_PlayerState.Multiplayer_PlayerState_C|GetSession%20Color _askotf_player_state) :!class /Script/Engine.MaterialInstanceDynamic))
    (:Is%20Not%20Valid
      (bind _returnvalue (Rendering|Material|CreateDynamicMaterialInstance "/Game/GameModes/KOTF/Blueprints/Flag/Outline/PP_OutlineCustomDepthOcclusion.PP_OutlineCustomDepthOcclusion" :!class /Script/Engine.KismetMaterialLibrary))
      (bind _output_get (Variables|Default|SetPP_Material _returnvalue))
      (Rendering|Material|SetVectorParameterValue _output_get "OutlineColor" (Variables|/Game/Multiplayer/Blueprints/Overrides/Multiplayer_PlayerState.Multiplayer_PlayerState_C|GetSession%20Color _askotf_player_state) :!class /Script/Engine.MaterialInstanceDynamic)))
  (bind _outactors (Actor|GetAllActorsOfClass "/Script/Engine.PostProcessVolume"))
  (for _array_element _outactors
    (bind _aspost_process_volume (Utilities|Casting|CastToPostProcessVolume _array_element))
    (Rendering|AddorUpdateBlendable _aspost_process_volume (Variables|Default|GetPP_Material) 1.0 :!class /Script/Engine.PostProcessVolume)))

(fn ConstructionScript
  (Utilities|FlowControl|Sequence
    (:then_0
      (Variables|Default|SetRespawnLocation (Transformation|GetActorTransform))
      (Transformation|SetRelativeLocationAndRotation (Variables|Default|GetPickup) (Variables|Modularity|GetPick-Up%20Location) (Variables|Modularity|GetPick-Up%20Rotation) false false)
      (Components|StaticMesh|SetStaticMesh (Variables|Default|GetPickup) (Variables|Modularity|GetPick-Up%20Mesh))
      (Variables|/Script/Engine.RotatingMovementComponent|SetRotationRate (Variables|Default|GetRotatingMovement) (Variables|Modularity|GetRotation%20Rate))
      (Transformation|SetRelativeScale3D (Variables|Default|GetPickup) (Variables|Modularity|GetPick-Up%20Scale)))
    (:then_1
      (Transformation|SetRelativeLocationAndRotation (Variables|Default|GetSphere) (Variables|Modularity|GetPick-Up%20Collision%20Location) (Variables|Modularity|GetPick-Up%20Collision%20Rotation) false false)
      (Transformation|SetRelativeScale3D (Variables|Default|GetSphere) (Variables|Modularity|GetPick-Up%20Collision%20Size)))))