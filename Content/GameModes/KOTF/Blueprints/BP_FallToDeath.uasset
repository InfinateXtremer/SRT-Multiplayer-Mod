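; A kill volume for the KOTF game mode that respawns any playable character falling into its box.
; On BeginPlay it caches the first BP_Flag_Gift in the level.
; If the overlapping player is the current flag holder, it respawns the flag before moving the player.
; Respawn teleports the player to the transform of a randomly chosen PlayerStart, without resetting or destroying the character.
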(event OnComponentBeginOverlap(Box)
  (params (OverlappedComponent :type Primitive%20Component%20Object%20Reference) (OtherActor :type Actor%20Object%20Reference) (OtherComp :type Primitive%20Component%20Object%20Reference) (OtherBodyIndex :type Integer) (bFromSweep :type Boolean) (SweepResult :type Hit%20Result%20Structure%20%28by%20ref%29))
  (bind _flag (Variables|Default|GetFlag))
  (bind _asbp_cps1999_playable (Utilities|Casting|CastToBP_CPS1999_Playable OtherActor))
  (if (== _asbp_cps1999_playable (Variables|/Game/GameModes/KOTF/Blueprints/Flag/Blueprints/BP_Flag_Gift.BP_Flag_Gift_C|GetCurrent%20Flag%20Holder _flag))
    (Default|RespawnFlag _flag)
    (CallFunction|RespawnPlayer _asbp_cps1999_playable)
    (else
      (CallFunction|RespawnPlayer _asbp_cps1999_playable))))

(event Custom|RespawnPlayer
  (params (Player :type BP%20CPS1999%20Playable%20Object%20Reference))
  ;[1 1 1] Gets all player starts and randomly selects one
  (bind _outactors (Actor|GetAllActorsOfClass "/Script/Engine.PlayerStart"))
  (bind _output_get (Variables|Default|SetRandomSpawnPoint (Math|Random|RandomInteger (Utilities|Array|Length _outactors))))
  (Transformation|SetActorTransform Player (Transformation|GetActorTransform (Utilities|Array|Get(acopy) _outactors _output_get))))

(event EventBeginPlay
  (bind _outactors (Actor|GetAllActorsOfClass "/Game/GameModes/KOTF/Blueprints/Flag/Blueprints/BP_Flag_Gift.BP_Flag_Gift_C"))
  (bind _asbp_flag_gift (Utilities|Casting|CastToBP_Flag_Gift (Utilities|Array|Get(acopy) _outactors)))
  (Variables|Default|SetFlag _asbp_flag_gift))

(fn ConstructionScript)