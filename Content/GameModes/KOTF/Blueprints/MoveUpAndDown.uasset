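; Scene component in the KOTF game mode, apparently meant to move the component it is attached to by a MoveHeight offset.
; BeginPlay stores the parent's world location plus that offset as the target Height.
; Tick compares the parent's location to Height but acts on neither result.
; The delta-time lerp that would move the parent is disconnected, so nothing moves, and no return motion exists.
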(event EventTick
  (params (DeltaSeconds :type Float%20%28single-precision%29))
  (if (Math|Vector|Equal(Vector) (Transformation|GetWorldLocation (Transformation|GetAttachParent)) (Variables|Default|GetHeight) 0.0001)
    _))

(event EventBeginPlay
  (Variables|Default|SetHeight (+ (Transformation|GetWorldLocation (Transformation|GetAttachParent)) (Variables|Default|GetMoveHeight))))