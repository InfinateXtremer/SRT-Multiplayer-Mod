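; BP_Flag_Gift is the carried flag of the KOTF game mode, scoring points for whoever holds it.
; Server-side overlap passes it to the touching player with a brief cooldown, while a multicast attaches it to their back, plays a sound and moves the custom-depth highlight.
; A looping server timer increments the holder's PlayerState points each second.
; At the score limit it plays an unreplicated win sound, then server-travels to restart the level.
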(event OnComponentBeginOverlap(Sphere)
  (params (OverlappedComponent :type Primitive%20Component%20Object%20Reference) (OtherActor :type Actor%20Object%20Reference) (OtherComp :type Primitive%20Component%20Object%20Reference) (OtherBodyIndex :type Integer) (bFromSweep :type Boolean) (SweepResult :type Hit%20Result%20Structure%20%28by%20ref%29))
  (Networking|SwitchHasAuthority
    (:Authority
      (bind _asbp_cps1999_playable (Utilities|Casting|CastToBP_CPS1999_Playable OtherActor))
      (CallFunction|PickupServer _asbp_cps1999_playable))))

(event Custom|PickupServer
  (params (Player :type BP%20CPS1999%20Playable%20Object%20Reference))
  (if (not (Variables|Default|GetInCooldown))
    (Variables|Default|SetInCooldown true)
    (CallFunction|PickupMulticast Player (Variables|Default|GetCurrent%20Flag%20Holder)) ; Tell everyone else someone has picked me up!
    (bind _output_get (Variables|Default|SetCurrent%20Flag%20Holder Player))
    (bind _askotf_player_state (Utilities|Casting|CastToKOTF_PlayerState (Variables|/Script/Engine.Pawn|GetPlayerState _output_get)))
    (Variables|Default|SetFlag%20Holder's%20State _askotf_player_state)
    (Utilities|FlowControl|Delay 2.0)
    (Variables|Default|SetInCooldown false)))

(event Custom|PickupMulticast
  (params (Player :type BP%20CPS1999%20Playable%20Object%20Reference) (PreviousPlayer :type BP%20CPS1999%20Playable%20Object%20Reference))
  (Utilities|IsValid PreviousPlayer
    (:Is%20Valid
      (Rendering|SetRenderCustomDepth (Variables|/Script/Engine.Character|GetMesh PreviousPlayer) false))
    (:Is%20Not%20Valid
      _))
  (Rendering|SetRenderCustomDepth (Variables|/Script/Engine.Character|GetMesh Player) true)
  (Transformation|AttachActorToActor self Player "socket_BackAttach_Upper" "SnapToTarget" "KeepRelative" "KeepRelative" true)
  (Audio|SpawnSoundAttached "/Game/GameModes/KOTF/Flag/Sound/PickedUp.PickedUp" (Variables|/Script/Engine.Character|GetMesh Player) "None" "0, 0, 0" "0, 0, 0" "SnapToTarget" false 1.0 1.0 0.0 "/Game/GameModes/KOTF/Flag/Sound/GeneralSpeech.GeneralSpeech"))

(event Custom|PointCounter
  (bind _flag_holder_s_state (Variables|Default|GetFlag%20Holder's%20State))
  (Utilities|IsValid _flag_holder_s_state
    (:Is%20Valid
      (if (== (Variables|/Game/GameModes/KOTF/MultiplayerMode/KOTF_PlayerState.KOTF_PlayerState_C|GetPoints _flag_holder_s_state) 60)
        (Utilities|FlowControl|DoOnce false
          (:Completed
            (Utilities|Time|ClearandInvalidateTimerbyHandle (stale EventBeginPlay _returnvalue))
            ;[1 1 1] Replicate This
            (Audio|PlaySound2D "/Game/GameModes/KOTF/Flag/Sound/cossack_sandvich.cossack_sandvich")
            (Utilities|FlowControl|Delay 1e+01)
            (bind _returnvalue (Game|GetCurrentLevelName true))
            (Development|ExecuteConsoleCommand (Utilities|String|Append "servertravel " _returnvalue))))
        (else
          (Variables|/Game/GameModes/KOTF/MultiplayerMode/KOTF_PlayerState.KOTF_PlayerState_C|SetPoints _flag_holder_s_state (+ 1 (Variables|/Game/GameModes/KOTF/MultiplayerMode/KOTF_PlayerState.KOTF_PlayerState_C|GetPoints _flag_holder_s_state))))))))

(event EventBeginPlay
  (Networking|SwitchHasAuthority
    (:Authority
      (bind _returnvalue (Utilities|Time|SetTimerbyEvent (delegate Custom|PointCounter) 1.0 true)))))

(fn ConstructionScript)

(fn OnRepinCooldown)

(fn OnRepTimer)

(fn OnRepPlayerwithFlag)

(fn OnRepPlayerState)

(fn OnRepHaveFlag?)