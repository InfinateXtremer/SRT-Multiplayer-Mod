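; Player controller for the KOTF multiplayer game mode that sets the KOTH_HUD on BeginPlay and handles release of the ChargeAttack input.
; On release it casts the controlled playable pawn's Ability System Component to GA_Spyro_Charge to end it.
; That cast targets the component rather than an ability instance, so the Crit_hit sound fallback is the expected result.
; Unconnected nodes for removing the charging effect and committing an ability never run.
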(event EventBeginPlay
  (Class|PlayerController|ClientSetHUD "/Game/GameModes/KOTF/MultiplayerMode/KOTH_HUD.KOTH_HUD_C"))

(event Input|ActionEvents|InputActionChargeAttack
  (params (Key :type Key%20Structure))
  (:Released
    (bind _asbp_cps1999_playable (Utilities|Casting|CastToBP_CPS1999_Playable (Pawn|GetControlledPawn)))
    (bind _asga_spyro_charge (Utilities|Casting|CastToGA_Spyro_Charge (Ability|GetAbilitySystemComponent _asbp_cps1999_playable))
      (:then
        (Ability|EndAbility _asga_spyro_charge))
      (:CastFailed
        (Audio|PlaySound2D "/Game/GameModes/KOTF/Flag/Sound/crit_hit.crit_hit")))))

(fn ConstructionScript
  (|CallParentFunction))