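; BP_Elevator is an interactable platform that moves vertically between its placed location and a point Height units above it.
; Interact calls MovePlatform, which plays or reverses a timeline that lerps the actor's location according to IsElevatorDown.
; A DoOnce blocks retriggering during travel, and GoDownAutomatically sends the platform back down after a short delay at the top.
; The sound playback nodes are disconnected and never run.
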(event Custom|MovePlatform
  (if (Variables|Default|GetInteractable?)
    (Utilities|FlowControl|DoOnce false :!label _label
      (:Completed
        (if (Variables|Default|GetIsElevatorDown?) :!label _label_2
          (bind (_direction _newtrack_0) (Timeline|Timeline_0 PlayFromStart)
            (:Update
              (Transformation|SetActorLocation (Math|Vector|Lerp(Vector) (Variables|Default|GetStartingPoint) (Variables|Default|GetEnd%20Point) _newtrack_0) false false))
            (:Finished
              (if (Utilities|Enum|Equal(Enum) _direction "Forward")
                (Variables|Default|SetIsElevatorDown? false)
                (if (Variables|Default|GetGoDownAutomatically?)
                  (Utilities|FlowControl|Delay 0.3)
                  (goto _label_2)
                  (else
                    (goto _label Reset)))
                (else
                  (Variables|Default|SetIsElevatorDown? true)
                  (goto _label Reset)))))
          (else
            (Timeline|Timeline_0 ReverseFromEnd)))))))

(event EventInteract
  (CallFunction|MovePlatform))

(fn ConstructionScript
  (bind _returnvalue (Transformation|GetActorLocation))
  (bind (_x _y _z) (Math|Vector|BreakVector _returnvalue))
  (Variables|Default|SetStartingPoint _returnvalue)
  (Variables|Default|SetEnd%20Point (Math|Vector|MakeVector _x _y (+ _z (Variables|Default|GetHeight)))))