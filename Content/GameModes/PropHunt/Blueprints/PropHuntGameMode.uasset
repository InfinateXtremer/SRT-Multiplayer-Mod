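; PropHuntGameMode is the game mode for Prop Hunt, assigning a role flag to the players after a fixed five-minute delay from BeginPlay.
; Its server spawn event spawns nothing itself; it loops over every BP_Proproller_Player and calls ServerSetPlayer with true or false.
; True requires the loop index to match a random integer, drawn inside the loop between zero and the negated player count.
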(event Custom|Server_SpawnPlayers
  (bind _outactors (Actor|GetAllActorsOfClass "/CharacterCommon/Controllers/BP_Proproller_Player.BP_Proproller_Player_C"))
  (for (_array_element _array_index) _outactors
    (if (== _array_index (Math|Random|RandomIntegerinRange 0 (- 0 (Utilities|Array|Length _outactors))))
      (Default|ServerSetPlayer _array_element true)
      (else
        (Default|ServerSetPlayer _array_element false)))))

(event EventBeginPlay
  (Utilities|FlowControl|Delay 3e+02)
  (CallFunction|ServerSpawnPlayers))

(fn ConstructionScript
  (|CallParentFunction))