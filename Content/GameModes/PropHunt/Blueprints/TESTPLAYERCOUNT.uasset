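; PropHunt test actor that displays the current player count on a TextRender component.
; Two seconds after BeginPlay it chains through GetPlayerCountServer to GetPlayerCount, which casts the game mode to MultiplayerMode and writes GetNumPlayers to the text.
; The count is read once, with no later refresh, and nothing is written if the cast fails.
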(event Custom|GetPlayerCount
  (bind _asmultiplayer_mode (Utilities|Casting|CastToMultiplayerMode (Game|GetGameMode)))
  (bind _returnvalue (Class|GameModeBase|GetNumPlayers _asmultiplayer_mode))
  (Rendering|Components|TextRender|SetText (Variables|Default|GetTextRender) (Utilities|Text|ToText(Integer) _returnvalue)))

(event Custom|GetPlayerCountServer
  (CallFunction|GetPlayerCount))

(event EventBeginPlay
  (Utilities|FlowControl|Delay 2.0)
  (CallFunction|GetPlayerCountServer))

(fn ConstructionScript)