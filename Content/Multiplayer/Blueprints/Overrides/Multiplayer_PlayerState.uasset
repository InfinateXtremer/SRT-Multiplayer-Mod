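; Multiplayer player state that holds a player's session name, color, avatar and avatar tint, and handles character swaps.
; SetDefault loads these values from the game instance, and a one-time Tick and RepNotifies push them to the controlled pawn through messages.
; SwapCharacter spawns one of five character classes at the current pawn's transform, destroys that pawn and possesses the new one.
; RaiseMapTravelWarning is empty, with its menu logic left unconnected.
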(event Custom|Change%20Name
  (params (New%20Name :type Text))
  (Variables|Info|SetSession%20Name New%20Name))

(event Custom|Swap%20Character
  (params (New%20Character :type PlayableCharacterEnum%20Enum :default "NewEnumerator0"))
  (bind _returnvalue (Components|GetOwner))
  (bind _returnvalue_2 (Utilities|Select :Index New%20Character :NewEnumerator0 "/Game/Multiplayer/Blueprints/MultiplayerCharacters/BP_Spyro_Multi.BP_Spyro_Multi_C" :NewEnumerator1 "/Game/Multiplayer/Blueprints/MultiplayerCharacters/BP_Sheila_Multi.BP_Sheila_Multi_C" :NewEnumerator3 "/Game/Multiplayer/Blueprints/MultiplayerCharacters/BP_SgtByrd_Multi.BP_SgtByrd_Multi_C" :NewEnumerator4 "/Game/Multiplayer/Blueprints/MultiplayerCharacters/BP_Bentley_Multi.BP_Bentley_Multi_C" :NewEnumerator5 "/Game/Multiplayer/Blueprints/MultiplayerCharacters/BP_Agent9_Multi.BP_Agent9_Multi_C"))
  (if (Utilities|Enum|NotEqual(Enum) New%20Character (Variables|Default|GetMultiplayer%20Character))
    (if (Utilities|IsValidClass _returnvalue_2)
      (bind _asplayer_controller (Utilities|Casting|CastToPlayerController _returnvalue))
      (bind _returnvalue_3 (Game|SpawnActorfromClass _returnvalue_2 (Transformation|GetActorTransform (Pawn|GetControlledPawn _asplayer_controller)) "AlwaysSpawn" _returnvalue 0))
      (Actor|DestroyActor (Pawn|GetControlledPawn _asplayer_controller))
      (bind _aspawn (Utilities|Casting|CastToPawn _returnvalue_3))
      (Pawn|Possess _asplayer_controller _aspawn)
      (Variables|Default|SetMultiplayer%20Character New%20Character))))

(event Custom|Change%20Avatar
  (params (New%20Avatar :type Name))
  (Variables|Info|SetSession%20Avatar New%20Avatar))

(event Custom|Change%20Avatar%20Tint
  (params (New%20Tint :type Boolean))
  (Variables|Info|SetSession%20Color%20Avatar New%20Tint))

(event Custom|Change%20Color
  (params (New%20Color :type Linear%20Color%20Structure :default "(R=1.000000,G=1.000000,B=1.000000,A=1.000000)"))
  (Variables|Info|SetSession%20Color New%20Color))

(event Custom|Set%20Default
  (bind _asmultiplayer_instance (Utilities|Casting|CastToMultiplayerInstance (Game|GetGameInstance)))
  (CallFunction|ChangeName (Utilities|Text|ToText(Name) (Variables|/Game/Multiplayer/Blueprints/Overrides/MultiplayerInstance.MultiplayerInstance_C|GetPersistent%20Display%20Name _asmultiplayer_instance)))
  (CallFunction|ChangeColor (Variables|/Game/Multiplayer/Blueprints/Overrides/MultiplayerInstance.MultiplayerInstance_C|GetPersistent%20Color _asmultiplayer_instance))
  (CallFunction|ChangeAvatar (Variables|/Game/Multiplayer/Blueprints/Overrides/MultiplayerInstance.MultiplayerInstance_C|GetPersistent%20Avatar _asmultiplayer_instance))
  (CallFunction|ChangeAvatarTint (Variables|/Game/Multiplayer/Blueprints/Overrides/MultiplayerInstance.MultiplayerInstance_C|GetPersistent%20Tint%20Avatar _asmultiplayer_instance)))

(event Custom|Raise%20Map%20Travel%20Warning)

(event EventTick
  (params (DeltaSeconds :type Float%20%28single-precision%29))
  (Utilities|FlowControl|DoOnce false
    (:Completed
      (Utilities|FlowControl|Sequence
        (:then_0
          (Networking|SwitchHasAuthority
            (:Authority
              (bind _asplayer_controller (Utilities|Casting|CastToPlayerController (Components|GetOwner)))
              (Variables|Default|SetControlled%20Pawn (Pawn|GetControlledPawn _asplayer_controller)))))
        (:then_1
          (Class|BICustomizationInterface|ChangeName(Message) (Variables|Default|GetControlled%20Pawn) (Variables|Info|GetSession%20Name))
          (Class|BICustomizationInterface|ChangeColor(Message) (Variables|Default|GetControlled%20Pawn) (Variables|Info|GetSession%20Color))
          (Class|BICustomizationInterface|ChangeAvatar(Message) (Variables|Default|GetControlled%20Pawn) (Variables|Info|GetSession%20Avatar))
          (Class|BICustomizationInterface|ChangeAvatarTint(Message) (Variables|Default|GetControlled%20Pawn) (Variables|Info|GetSession%20Color%20Avatar)))))))

(fn ConstructionScript)

(fn OnRepName
  (bind _asbp_oldtroller_player (Utilities|Casting|CastToBP_Oldtroller_Player (Components|GetOwner)))
  (Class|BICustomizationInterface|ChangeName(Message) (Pawn|GetControlledPawn _asbp_oldtroller_player) (Variables|Info|GetSession%20Name)))

(fn OnRepColor
  (bind _asbp_oldtroller_player (Utilities|Casting|CastToBP_Oldtroller_Player (Components|GetOwner)))
  (Class|BICustomizationInterface|ChangeColor(Message) (Pawn|GetControlledPawn _asbp_oldtroller_player) (Variables|Info|GetSession%20Color)))

(fn OnRepColorAvatar
  (bind _asbp_oldtroller_player (Utilities|Casting|CastToBP_Oldtroller_Player (Components|GetOwner)))
  (Class|BICustomizationInterface|ChangeAvatarTint(Message) (Pawn|GetControlledPawn _asbp_oldtroller_player) (Variables|Info|GetSession%20Color%20Avatar)))

(fn OnRepSessionAvatar
  (bind _asbp_oldtroller_player (Utilities|Casting|CastToBP_Oldtroller_Player (Components|GetOwner)))
  (Class|BICustomizationInterface|ChangeAvatar(Message) (Pawn|GetControlledPawn _asbp_oldtroller_player) (Variables|Info|GetSession%20Avatar)))