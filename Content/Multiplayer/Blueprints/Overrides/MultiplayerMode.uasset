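; Multiplayer game mode that initializes the state of each player who logs in.
; On PostLogin it casts the new player's PlayerState to Multiplayer_PlayerState and calls SetDefault on it.
; BeginPlay and the controller swap event are empty.
; Unconnected leftover logic would hide the menu's map travel warning and set SessionName from the player's name, but never runs.
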(event EventPostLogin
  (params (NewPlayer :type Player%20Controller%20Object%20Reference))
  (bind _asmultiplayer_player_state (Utilities|Casting|CastToMultiplayer_PlayerState (Variables|/Script/Engine.Controller|GetPlayerState NewPlayer)))
  (Default|SetDefault _asmultiplayer_player_state))

(event EventBeginPlay)

(event EventOnSwapPlayerControllers
  (params (OldPC :type Player%20Controller%20Object%20Reference) (NewPC :type Player%20Controller%20Object%20Reference)))

(fn ConstructionScript
  (|CallParentFunction))