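; Player controller override for multiplayer that toggles the multiplayer menu with the M key.
; A macro fetches the menu from the MultiplayerInstance game instance and flips its widget's visibility with a FlipFlop.
; The mouse cursor follows that visibility, and the menu resets whenever it is hidden.
; A disconnected, similar toggle for a mod loader menu remains in the graph but never runs.
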(event Input|KeyboardEvents|M
  (params (Key :type Key%20Structure))
  (:Pressed
    (bind (_menu _isvisible) (Utilities|NewMacro0 (Variables|/Game/Multiplayer/Blueprints/UserInterface/MultiplayerMenu.MultiplayerMenu_C|GetMultiplayerMenu (stale _menu)))
      (:Out
        (Utilities|FlowControl|Sequence
          (:then_0
            (if (not _isvisible)
              (Default|Reset _menu)))
          (:then_1
            (Variables|/Script/Engine.PlayerController|SetbShowMouseCursor self (or _isvisible false))))))))

(fn ConstructionScript
  (|CallParentFunction))