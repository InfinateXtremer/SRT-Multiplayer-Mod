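; Game instance for multiplayer that holds the local player's profile, session hosting state and menu widget.
; Init loads display name, color and avatar settings from a save slot, and Shutdown writes them back, creating the save object if needed.
; A hosting flag guards session creation and destruction, which open the lobby and global persistent level respectively.
; GetMenu lazily creates and caches the multiplayer menu, re-adding it to the viewport when absent.
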(event Custom|Host%20Multplayer%20Session
  (if (not (Variables|Multiplayer|GetIs%20Hosting%20Session))
    (Variables|Multiplayer|SetIs%20Hosting%20Session true)
    (|Session (Game|GetPlayerController 0) 0 false
      (:then
        (Game|OpenLevel(byName) "Lobby" true "listen")))))

(event Custom|Close%20Multiplayer%20Session
  (if (Variables|Multiplayer|GetIs%20Hosting%20Session)
    (Variables|Multiplayer|SetIs%20Hosting%20Session false)
    (|DestroySession (Game|GetPlayerController 0)
      (:then
        (Game|OpenLevel(byName) "GlobalPersistentLevel")))))

(event EventShutdown
  (Utilities|IsValid (Variables|Multiplayer|Persistent|GetLocal%20Persistent%20Multiplayer%20Data)
    (:Is%20Valid
      _)
    (:Is%20Not%20Valid
      (bind _returnvalue (SaveGame|CreateSaveGameObject "/Game/Multiplayer/Blueprints/MultiplayerSave.MultiplayerSave_C"))
      (bind _output_get (Variables|Multiplayer|Persistent|SetLocal%20Persistent%20Multiplayer%20Data _returnvalue))))
  (Variables|/Game/Multiplayer/Blueprints/MultiplayerSave.MultiplayerSave_C|SetDisplay%20Name _output_get (Variables|Multiplayer|Persistent|GetPersistent%20Display%20Name))
  (Variables|/Game/Multiplayer/Blueprints/MultiplayerSave.MultiplayerSave_C|SetColor _output_get (Variables|Multiplayer|Persistent|GetPersistent%20Color))
  (Variables|/Game/Multiplayer/Blueprints/MultiplayerSave.MultiplayerSave_C|SetAvatar%20Name _output_get (Variables|Multiplayer|Persistent|GetPersistent%20Avatar))
  (Variables|/Game/Multiplayer/Blueprints/MultiplayerSave.MultiplayerSave_C|SetColor%20Avatar _output_get (Variables|Multiplayer|Persistent|GetPersistent%20Tint%20Avatar))
  (SaveGame|SaveGametoSlot _output_get "Multiplayer"))

(event EventInit
  (bind _returnvalue (SaveGame|LoadGamefromSlot "Multiplayer"))
  (bind _asmultiplayer_save (Utilities|Casting|CastToMultiplayerSave _returnvalue))
  (bind _output_get (Variables|Multiplayer|Persistent|SetLocal%20Persistent%20Multiplayer%20Data _asmultiplayer_save))
  (Utilities|IsValid _output_get
    (:Is%20Valid
      (Variables|Multiplayer|Persistent|SetPersistent%20Display%20Name (Variables|/Game/Multiplayer/Blueprints/MultiplayerSave.MultiplayerSave_C|GetDisplay%20Name _output_get))
      (Variables|Multiplayer|Persistent|SetPersistent%20Color (Variables|/Game/Multiplayer/Blueprints/MultiplayerSave.MultiplayerSave_C|GetColor _output_get))
      (Variables|Multiplayer|Persistent|SetPersistent%20Avatar (Variables|/Game/Multiplayer/Blueprints/MultiplayerSave.MultiplayerSave_C|GetAvatar%20Name _output_get))
      (Variables|Multiplayer|Persistent|SetPersistent%20Tint%20Avatar (Variables|/Game/Multiplayer/Blueprints/MultiplayerSave.MultiplayerSave_C|GetColor%20Avatar _output_get)))))

(fn GetMenu
  (Utilities|IsValid (Variables|Multiplayer|GetMultiplayer%20Menu)
    (:Is%20Valid
      (if (UserInterface|Viewport|IsinViewport (Variables|Multiplayer|GetMultiplayer%20Menu))
        _
        (else
          (UserInterface|Viewport|AddtoViewport (Variables|Multiplayer|GetMultiplayer%20Menu) 1000)))
      (return (Variables|Multiplayer|GetMultiplayer%20Menu)))
    (:Is%20Not%20Valid
      (bind _returnvalue (UserInterface|CreateWidget "/Game/Multiplayer/Blueprints/UserInterface/MultiplayerMenu.MultiplayerMenu_C" (Game|GetPlayerController 0)))
      (UserInterface|Viewport|AddtoViewport _returnvalue 1000)
      (bind _output_get (Variables|Multiplayer|SetMultiplayer%20Menu _returnvalue))
      (return _output_get))))