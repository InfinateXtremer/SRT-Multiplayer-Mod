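; Multiplayer Spyro character that shows each player's chosen avatar, tint and colored name tag.
; Avatar changes look up mesh and materials in the game instance's Avatars map, falling back to classic Spyro.
; SwapMaterialSet builds dynamic body and eye materials, tinting the body with the name tag color when enabled.
; Each tick turns the tag toward the camera; once the PlayerState arrives, the local player's own tag is hidden.
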(event Custom|Update%20Avatar%20Tint
  (params (Tint :type Boolean))
  (bind _output_get (Variables|Default|SetTinted Tint))
  (bind _asmultiplayer_player_state (Utilities|Casting|CastToMultiplayer_PlayerState (Variables|Default|GetPlayerState)))
  (Utilities|SwapMaterialSet _output_get (Variables|/Game/Multiplayer/Blueprints/Overrides/Multiplayer_PlayerState.Multiplayer_PlayerState_C|GetSession%20Avatar _asmultiplayer_player_state)))

(event Custom|Update%20Color
  (params (New%20Color :type Linear%20Color%20Structure))
  (Rendering|Components|TextRender|SetTextRenderColor (Variables|Default|GetName%20Tag) (Math|Conversions|ToColor(LinearColor) New%20Color))
  (if (Variables|Default|GetTinted)
    (Rendering|Material|SetVectorParameterValue (Variables|Default|GetSkin) "Tint Color" New%20Color :!class /Script/Engine.MaterialInstanceDynamic)))

(event Custom|Update%20Name
  (params (New%20Name :type Text))
  (Rendering|Components|TextRender|SetText (Variables|Default|GetName%20Tag) New%20Name))

(event Custom|Update%20Avatar
  (params (New%20Avatar :type Name))
  (bind _asmultiplayer_instance (Utilities|Casting|CastToMultiplayerInstance (Game|GetGameInstance)))
  (Utilities|FlowControl|Sequence
    (:then_0
      (Class|SkinnedMeshComponent|SetSkeletalMesh (Variables|Character|GetMesh) (Utilities|Struct|BreakSpyroAvatar (select (.ReturnValue (Utilities|Map|Find (Variables|/Game/Multiplayer/Blueprints/Overrides/MultiplayerInstance.MultiplayerInstance_C|GetAvatars _asmultiplayer_instance) New%20Avatar)) (.Value (Utilities|Map|Find (Variables|/Game/Multiplayer/Blueprints/Overrides/MultiplayerInstance.MultiplayerInstance_C|GetAvatars _asmultiplayer_instance) New%20Avatar)) (Utilities|Struct|MakeSpyroAvatar "/CPS1999_Spyro/Mesh/SK_CPS1999_Spyro.SK_CPS1999_Spyro" "/CPS1999_Spyro/Materials/MI_CPS1999_Spyro_Body.MI_CPS1999_Spyro_Body" "/CPS1999_Spyro/Materials/MI_CPS1999_Spyro_Greyscale.MI_CPS1999_Spyro_Greyscale" "/CPS1999_Spyro/Materials/MI_CPS1999_Spyro_Eye_L.MI_CPS1999_Spyro_Eye_L" "/CPS1999_Spyro/Materials/MI_CPS1999_Spyro_Eye_R.MI_CPS1999_Spyro_Eye_R"))) false))
    (:then_1
      (Utilities|SwapMaterialSet (Variables|Default|GetTinted) New%20Avatar))))

(event EventTick
  (params (DeltaSeconds :type Float%20%28single-precision%29))
  ;[1 1 1] Fixes Glide/Half Breaks Charge
  (|CallParentFunction DeltaSeconds))

(event EventAddonTick
  (params (Delta%20Seconds :type Float%20%28single-precision%29))
  (bind _name_tag (Variables|Default|GetName%20Tag))
  (Utilities|FlowControl|Sequence
    (:then_0
      (bind _player_state (Utilities|PollPlayerState)
        (:Player%20State%20Retreived
          (if (Pawn|IsLocallyControlled)
            (bind _asmultiplayer_player_state (Utilities|Casting|CastToMultiplayer_PlayerState _player_state))
            (Rendering|SetVisibility _name_tag false false)
            (Rendering|Components|TextRender|SetText _name_tag (Variables|/Game/Multiplayer/Blueprints/Overrides/Multiplayer_PlayerState.Multiplayer_PlayerState_C|GetSession%20Name _asmultiplayer_player_state))))))
    (:then_1
      ;[1 1 1] Face Tag to Camera
      (Transformation|SetWorldRotation (Variables|Default|GetName%20Tag) (Math|Rotator|FindLookatRotation (Transformation|GetActorForwardVector (Game|GetPlayerCameraManager 0)) (Math|Vector|MakeVector 0.0 0.0 0.0)) false true))))

(event EventChangeAvatar
  (params (New%20Avatar :type Name :default "None"))
  (CallFunction|UpdateAvatar New%20Avatar))

(event EventChangeName
  (params (New%20Name :type Text))
  (CallFunction|UpdateName New%20Name))

(event EventChangeColor
  (params (New%20Color :type Linear%20Color%20Structure))
  (CallFunction|UpdateColor New%20Color))

(event EventChangeAvatarTint
  (params (New%20Tint :type Boolean))
  (CallFunction|UpdateAvatarTint New%20Tint))

(event EventAddononBeginPlay)

(fn ConstructionScript
  (|CallParentFunction))